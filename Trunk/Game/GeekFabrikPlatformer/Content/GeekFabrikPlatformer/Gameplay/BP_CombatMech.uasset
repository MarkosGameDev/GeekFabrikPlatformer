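; BP_CombatMech is a player-controlled mech character with movement, look and jump controls.
; BeginPlay registers its Enhanced Input mapping context and applies an initial camera pitch offset.
; Movement follows the control rotation, and look input drives controller yaw and pitch.
; Jumping plays a timeline that raises gravity scale mid-curve for a heavier fall and restores it on finish, while Tick derives IsJumping from ground state.
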(event `self.ReceiveBeginPlay`
  (`|ExecutionSequence`
    (:`then_0`
      (bind _asplayer_controller (cast `PlayerController` (`self.GetController`)))
      (bind _returnvalue (pcsubsystem `EnhancedInputLocalPlayerSubsystem` _asplayer_controller))
      (`/Engine/EditorBlueprintResources/StandardMacros.IsValid` _returnvalue
        (:`Is Valid`
          (`EnhancedInputSubsystemInterface.AddMappingContext` _returnvalue "/Game/GeekFabrikPlatformer/Gameplay/Input/IMC_CombatMech.IMC_CombatMech" 0 (struct)))))
    (:`then_1`
      (`self.AddControllerPitchInput` 13.0))))

(event `EnhancedInput|/Game/GeekFabrikPlatformer/Gameplay/Input/Actions/IA_CombatMech`
  (params (ActionValue :type "Vector2D Structure") (ElapsedSeconds :type "Float (double-precision)") (TriggeredSeconds :type "Float (double-precision)") (InputAction :type "InputAction Object Reference" :default "/Game/GeekFabrikPlatformer/Gameplay/Input/Actions/IA_CombatMech.IA_CombatMech"))
  (bind (_returnvalue_roll _returnvalue_pitch _returnvalue_yaw) (`KismetMathLibrary.BreakRotator` (`self.GetControlRotation`)))
  (bind (_returnvalue_roll_2 _returnvalue_pitch_2 _returnvalue_yaw_2) (`KismetMathLibrary.BreakRotator` (`self.GetControlRotation`)))
  ;[1 1 1] Comment
  (:`Triggered`
    (`self.AddMovementInput` (`KismetMathLibrary.GetRightVector` (`KismetMathLibrary.MakeRotator` _returnvalue_roll_2 0.0 _returnvalue_yaw_2)) ActionValue_X)
    (`self.AddMovementInput` (`KismetMathLibrary.GetForwardVector` (`KismetMathLibrary.MakeRotator` 0.0 0.0 _returnvalue_yaw)) ActionValue_Y)))

(event `EnhancedInput|/Game/GeekFabrikPlatformer/Gameplay/Input/Actions/IA_Look`
  (params (ActionValue :type "Vector2D Structure") (ElapsedSeconds :type "Float (double-precision)") (TriggeredSeconds :type "Float (double-precision)") (InputAction :type "InputAction Object Reference" :default "/Game/GeekFabrikPlatformer/Gameplay/Input/Actions/IA_Look.IA_Look"))
  (:`Triggered`
    (`self.AddControllerYawInput` ActionValue_X)
    (`self.AddControllerPitchInput` ActionValue_Y)))

(event `EnhancedInput|/Game/GeekFabrikPlatformer/Gameplay/Input/Actions/IA_Jump`
  (params (ActionValue :type Boolean) (ElapsedSeconds :type "Float (double-precision)") (TriggeredSeconds :type "Float (double-precision)") (InputAction :type "InputAction Object Reference" :default "/Game/GeekFabrikPlatformer/Gameplay/Input/Actions/IA_Jump.IA_Jump"))
  (:`Started`
    (set `self.isJumping` true)
    (`self.Jump`)
    (`Timeline|JumpTimeLine` :!via `PlayFromStart`
      (:`Finished`
        (set `CharacterMovementComponent.GravityScale` 1.0 (`self.CharacterMovement`)))
      (:`OnReachedMidOfTheCurve`
        (set `CharacterMovementComponent.GravityScale` 2.0 (`self.CharacterMovement`)))))
  (:`Completed`
    (`self.StopJumping`)))

(event `self.ReceiveTick`
  (params (DeltaSeconds :type "Float (single-precision)"))
  (set `self.isJumping` (not (`NavMovementComponent.IsMovingOnGround` (`self.CharacterMovement`)))))

(fn `UserConstructionScript`)