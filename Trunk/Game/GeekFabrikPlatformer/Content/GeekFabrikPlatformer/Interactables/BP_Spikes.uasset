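; BP_Spikes is a spike hazard for the platformer that damages the player when its overlap handling runs.
; It overrides HandleOverlap, calls the parent, then casts player controller 0 to PC_Gameplay and applies one point of damage to that controller rather than a pawn.
; Debug prints in Portuguese show the controller's Life before and after the damage.
; The standard event and construction graphs add no logic.
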(fn `HandleOverlap`
  (`parent.HandleOverlap`)
  (bind _aspc_gameplay (cast `/Game/GeekFabrikPlatformer/Gameplay/PC_Gameplay` (`GameplayStatics.GetPlayerController` 0)))
  (bind _returnvalue (`KismetStringLibrary.Conv_IntToString` (`/Game/GeekFabrikPlatformer/Gameplay/PC_Gameplay.Life` _aspc_gameplay)))
  (`KismetSystemLibrary.PrintString` (`KismetStringLibrary.Concat_StrStr` "Vida antes era: " _returnvalue))
  (`GameplayStatics.ApplyDamage` _aspc_gameplay 1.0)
  (`KismetSystemLibrary.PrintString` (`KismetStringLibrary.Concat_StrStr` "Vida é: " _returnvalue) true true (struct :`R` 0.98115 :`G` 1.0 :`B` 0.048941 :`A` 1.0)))

(fn `UserConstructionScript`
  (`parent.UserConstructionScript`))